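; BP_P38_Pawn is a player-controlled P-38 aircraft pawn that flies forward continuously.
; Each tick it spins the left and right propellers at a fixed rate and adds full movement input along its forward vector.
; Roll and Pitch axis inputs are clamped and scaled by RotationSpeed and delta time, then applied as local rotation, so steering changes the flight direction.
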(event `self.ReceiveTick`
  (params (DeltaSeconds :type "Float (single-precision)"))
  (`SceneComponent.K2_AddLocalRotation` (`self.RightPropeller`) (`KismetMathLibrary.MakeRotator` (* 1000.0 (`GameplayStatics.GetWorldDeltaSeconds`))) false false)
  (`SceneComponent.K2_AddLocalRotation` (`self.LeftPropeller`) (`KismetMathLibrary.MakeRotator` (* 1000.0 (`GameplayStatics.GetWorldDeltaSeconds`))) false false)
  (`self.AddMovementInput` (`self.GetActorForwardVector`)))

(event `InputAxis|Roll`
  (params (AxisValue :type "Float (single-precision)"))
  (`self.K2_AddActorLocalRotation` (`KismetMathLibrary.MakeRotator` (* (`KismetMathLibrary.ClampAngle` AxisValue -1.0 1.0) (`self.RotationSpeed`) (`GameplayStatics.GetWorldDeltaSeconds`)))))

(event `InputAxis|Pitch`
  (params (AxisValue :type "Float (single-precision)"))
  (`self.K2_AddActorLocalRotation` (`KismetMathLibrary.MakeRotator` 0.0 (* (`KismetMathLibrary.ClampAngle` AxisValue -1.0 1.0) (`self.RotationSpeed`) (`GameplayStatics.GetWorldDeltaSeconds`)))))

(fn `UserConstructionScript`)